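; BP_MeatCreature is a creature Blueprint that displays its needs and current AI state on an attached status widget.
; BeginPlay caches the progress bars and state text from WBP_CreatureStats, along with the player camera manager.
; Each Tick turns the widget toward the camera and polls the creature's values, showing Hunger and Thirst inverted, Randy directly, and the state name from AIComponent.
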(event `self.ReceiveBeginPlay`
  (bind _returnvalue (`GameplayStatics.GetPlayerCameraManager` 0))
  (bind _aswbp_creature_stats (cast `/Game/UI/WBP_CreatureStats` (`WidgetComponent.GetWidget` (`self.Widget Status`))))
  (set `self.PB Hunger` (`/Game/UI/WBP_CreatureStats.PB_Hunger` _aswbp_creature_stats))
  (set `self.PB Thirst` (`/Game/UI/WBP_CreatureStats.PB_Thirst` _aswbp_creature_stats))
  (set `self.PB Randyness` (`/Game/UI/WBP_CreatureStats.PB_Randyness` _aswbp_creature_stats))
  (set `self.TB State` (`/Game/UI/WBP_CreatureStats.TB_State` _aswbp_creature_stats))
  (`/Engine/EditorBlueprintResources/StandardMacros.IsValid` _returnvalue
    (:`Is Valid`
      (set `self.Camera Manager` _returnvalue))))

(event `self.ReceiveTick`
  (params (DeltaSeconds :type "Float (single-precision)"))
  (`|ExecutionSequence`
    (:`then_0`
      (`SceneComponent.K2_SetWorldRotation` (`self.Widget Status`) (`KismetMathLibrary.FindLookAtRotation` (`SceneComponent.K2_GetComponentLocation` (`self.Widget Status`)) (`PlayerCameraManager.GetCameraLocation` (`self.Camera Manager`))) false false))
    (:`then_1`
      (`ProgressBar.SetPercent` (`self.PB Hunger`) (/ (`KismetMathLibrary.Conv_IntToDouble` (- (`self.Hunger`) 100)) -100.0))
      (`ProgressBar.SetPercent` (`self.PB Thirst`) (/ (`KismetMathLibrary.Conv_IntToDouble` (- (`self.Thirst`) 100)) -100.0))
      (`ProgressBar.SetPercent` (`self.PB Randyness`) (/ (`KismetMathLibrary.Conv_IntToDouble` (`self.Randy`)) 100.0))
      (set `TextBlock.Text` (`KismetTextLibrary.Conv_StringToText` (`|GetEnumeratorNameAsString` (`CreatureState.StateName` (`AIComponent.CurrentCreatureState` (`self.AIComponent`))))) (`self.TB State`)))))

(fn `UserConstructionScript`)