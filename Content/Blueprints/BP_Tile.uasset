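; BP_Tile is a tile Blueprint that updates its cube's look and collision when its tile type is set.
; SetTileType calls the parent implementation, then selects a water, land or plant material from Type, with Obstacle sharing the water material.
; Obstacle tiles get query-only collision, while Water, Land and Plant tiles are probe-only.
; Tick, overlap and construction script are empty.
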(event `self.SetTileType`
  (params (NewType :type "ETileType Enum" :default "Water"))
  (`parent.SetTileType` NewType)
  (`PrimitiveComponent.SetMaterial` (`self.Cube`) 0 (select `ETileType` (`self.Type`) :`Water` "/Game/Materials/Tiles/M_Water.M_Water" :`Obstacle` "/Game/Materials/Tiles/M_Water.M_Water" :`Land` "/Game/Materials/Tiles/M_Land.M_Land" :`Plant` "/Game/Materials/Tiles/M_Plant.M_Plant" :!type "MaterialInterface Object Reference"))
  (switch `ETileType` (`self.Type`)
    (:`Water`
      (`PrimitiveComponent.SetCollisionEnabled` (`self.Cube`) "ProbeOnly" :!label _label))
    (:`Obstacle`
      (`PrimitiveComponent.SetCollisionEnabled` (`self.Cube`) "QueryOnly"))
    (:`Land`
      (goto _label))
    (:`Plant`
      (goto _label))))

(fn `UserConstructionScript`)