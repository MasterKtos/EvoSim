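; Map manager that builds the tile map from a character string at BeginPlay and spawns a test animal on the origin tile.
; StringToMapArray turns W, O, L and P into water, obstacle, land and plant entries, which feed GenerateMap with BP_Tile as prefab.
; Tick calls UpdateTiles every frame.
; SetNewTarget retries random eight-way neighbour picks until it gets a valid tile other than the old one.
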(event `self.ReceiveBeginPlay`
  (set `self.TilePrefab` "/Game/Blueprints/BP_Tile.BP_Tile_C")
  (bind _maparray (`self.StringToMapArray` (`self.StringMap0`)))
  (if (`KismetArrayLibrary.Array_IsNotEmpty` _maparray)
    (`self.GenerateMap` (make `InitialParameters` _maparray 10))
    (bind _returnvalue (`self.GetTileFromCoords` 0))
    (`|SpawnActorFromClass` "/Game/Blueprints/BP_AnimalTest.BP_AnimalTest_C" (`KismetMathLibrary.MakeTransform` (`self.K2_GetActorLocation` _returnvalue)) "AlwaysSpawn" "MultiplyWithRoot" null _returnvalue self null)))

(event `self.ReceiveTick`
  (params (DeltaSeconds :type "Float (single-precision)"))
  (`self.UpdateTiles`))

(fn `SetNewTarget`
  (params (OldTile :type "Tile Object Reference"))
  (returns (NewTile :type "Tile Object Reference"))
  (locals (ChosenTile :type "Tile Object Reference"))
  (while (or (== OldTile (`local.ChosenTile`)) (not (`KismetSystemLibrary.IsValid` (`local.ChosenTile`))))
    (set `local.ChosenTile` (`Tile.GetNeighbour` (`local.OldTile`) (select `int` (`KismetMathLibrary.RandomIntegerInRange` 0 7) :`0` "N" :`1` "NE" :`2` "E" :`3` "SE" :`4` "S" :`5` "SW" :`6` "W" :`7` "NW" :!type "EDirection Enum"))))
  (return (`local.ChosenTile`)))

(fn `StringToMapArray`
  (params (InputString :type String))
  (returns (MapArray :type "Array of ETileType Enum"))
  (locals (OutputMapArray :type "Array of ETileType Enum"))
  (`KismetSystemLibrary.PrintString` InputString)
  (for _array_element (`KismetStringLibrary.GetCharacterArrayFromString` InputString)
    (switch `string` _array_element
      (:`W`
        (`KismetArrayLibrary.Array_Add` (`local.OutputMapArray`) "Water"))
      (:`O`
        (`KismetArrayLibrary.Array_Add` (`local.OutputMapArray`) "Obstacle"))
      (:`L`
        (`KismetArrayLibrary.Array_Add` (`local.OutputMapArray`) "Land"))
      (:`P`
        (`KismetArrayLibrary.Array_Add` (`local.OutputMapArray`) "Plant"))))
  (return (`local.OutputMapArray`)))

(fn `UserConstructionScript`)